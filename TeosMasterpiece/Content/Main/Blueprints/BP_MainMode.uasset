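; BP_MainMode runs the enemy wave spawning and tracks a play timer that advances only while player controls are enabled.
; BeginPlay collects actors tagged EnemySpawn as spawn points and caches the BP_Player reference.
; Tick runs a spawn countdown, and while the enemy count is under its cap, multiplies the truncated wave size by DifficultyScale and spawns BP_Hannya at random points.
; The cap is checked once per wave, so waves can overshoot it.
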(event `self.ReceiveBeginPlay`
  (bind _outactors (`GameplayStatics.GetAllActorsWithTag` "EnemySpawn"))
  (for _array_element _outactors
    (`KismetArrayLibrary.Array_Add` (`self.SpawnPoints`) _array_element)
    (bind _asbp_player (cast `/Game/Main/Blueprints/BP_Player` (`GameplayStatics.GetPlayerPawn` 0)))
    (set `self.PlayRef` _asbp_player)))

(event `self.ReceiveTick`
  (params (DeltaSeconds :type "Float (single-precision)"))
  (if (not (`/Game/Main/Blueprints/BP_Player.DisableControls` (`self.PlayRef`)))
    (set `self.Timer` (+ DeltaSeconds (`self.Timer`))))
  (bind _output_get (set `self.SpawnTimer` (- (`self.SpawnTimer`) DeltaSeconds)))
  (if (<= _output_get 0.0)
    (set `self.SpawnTimer` (`self.SpawnTime`))
    (if (< (`self.EnemiesOnMap`) (`self.MaxEnemies`))
      (set `self.EnemiesToSpawn` (`KismetMathLibrary.FTrunc` (* (`self.EnemiesToSpawn`) (`self.DifficultyScale`))))
      (for _ (range (+ (`self.EnemiesToSpawn`) 1))
        (`|SpawnActorFromClass` "/Game/Main/Blueprints/Enemies/BP_Hannya.BP_Hannya_C" (`KismetMathLibrary.MakeTransform` (`self.K2_GetActorLocation` (`KismetArrayLibrary.Array_Random` (`self.SpawnPoints`)))) "Undefined" "OverrideRootScale" null null)
        (set `self.EnemiesOnMap` (+ (`self.EnemiesOnMap`) 1))))))

(fn `UserConstructionScript`)