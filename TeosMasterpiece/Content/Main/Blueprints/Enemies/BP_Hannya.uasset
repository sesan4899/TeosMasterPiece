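; BP_Hannya is a flying enemy that homes in on the player, deals damage on overlap and destroys itself.
; Each tick it retargets its randomly capped ProjectileMovement at the player capsule, adds a jittered cosine vertical bob and faces its velocity.
; Any damage fractures its Destructible with radial damage, decrements BP_MainMode's EnemiesOnMap and destroys it after a delay.
; Destruction by player contact skips that count update.
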(event `self.ReceiveBeginPlay`
  (set `ProjectileMovementComponent.MaxSpeed` (`KismetMathLibrary.RandomFloatInRange` 800.0 1000.0) (`self.ProjectileMovement`)))

(event `self.ReceiveTick`
  (params (DeltaSeconds :type "Float (single-precision)"))
  (bind _asbp_player (cast `/Game/Main/Blueprints/BP_Player` (`GameplayStatics.GetPlayerPawn` 0)))
  (set `ProjectileMovementComponent.HomingTargetComponent` (`Character.CapsuleComponent` _asbp_player) (`self.ProjectileMovement`))
  (`self.Sinus Movement`)
  (`self.Rotation`))

(event `self.DamageBox.OnComponentBeginOverlap`
  (params (OverlappedComponent :type "PrimitiveComponent Object Reference") (OtherActor :type "Actor Object Reference") (OtherComp :type "PrimitiveComponent Object Reference") (OtherBodyIndex :type Integer) (bFromSweep :type Boolean) (SweepResult :type "HitResult Structure (by ref)"))
  (if (== OtherActor (`GameplayStatics.GetPlayerPawn` 0))
    (`GameplayStatics.ApplyDamage` OtherActor 1.0)
    (`self.K2_DestroyActor`)))

(event `self.ReceiveAnyDamage`
  (params (Damage :type "Float (single-precision)") (DamageType :type "DamageType Object Reference") (InstigatedBy :type "Controller Object Reference") (DamageCauser :type "Actor Object Reference"))
  (`self.RadialDamageApply`)
  (`self.Update Game Mode`)
  (`KismetSystemLibrary.Delay` 5.0)
  (`self.K2_DestroyActor`))

(event `RadialDamageApply`
  (bind _destructible (`self.Destructible`))
  (`DestructibleComponent.ApplyRadiusDamage` _destructible 100.0 (`SceneComponent.K2_GetComponentLocation` _destructible) 100.0 100.0 false))

(fn `Rotation`
  (bind _returnvalue (`self.K2_GetActorLocation`))
  (`self.K2_SetActorRotation` (`KismetMathLibrary.FindLookAtRotation` _returnvalue (+ _returnvalue (`self.GetVelocity`)))))

(fn `Sinus Movement`
  (`SceneComponent.K2_AddRelativeLocation` (`self.DefaultSceneRoot`) (`KismetMathLibrary.MakeVector` 0.0 0.0 (* (`KismetMathLibrary.Cos` (`self.GetGameTimeSinceCreation`)) (`KismetMathLibrary.RandomFloatInRange` 0.25 0.75))) false false))

(fn `Update Game Mode`
  (bind _asbp_main_mode (cast `/Game/Main/Blueprints/BP_MainMode` (`GameplayStatics.GetGameMode`)))
  (set `/Game/Main/Blueprints/BP_MainMode.EnemiesOnMap` (- (`/Game/Main/Blueprints/BP_MainMode.EnemiesOnMap` _asbp_main_mode) 1) _asbp_main_mode))

(fn `UserConstructionScript`)