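; BP_Deathplane is a trigger volume that returns the player to a spawn point when they enter it.
; When the player pawn overlaps the Box, it casts to BP_Player and fades the camera out, holding when finished.
; After a short delay it teleports the player to the referenced Spawnpoint's location and rotation, then fades the camera back in.
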(event `self.Box.OnComponentBeginOverlap`
  (params (OverlappedComponent :type "PrimitiveComponent Object Reference") (OtherActor :type "Actor Object Reference") (OtherComp :type "PrimitiveComponent Object Reference") (OtherBodyIndex :type Integer) (bFromSweep :type Boolean) (SweepResult :type "HitResult Structure (by ref)"))
  (bind _returnvalue (`GameplayStatics.GetPlayerPawn` 0))
  (bind _spawnpoint (`self.Spawnpoint`))
  (if (== OtherActor _returnvalue)
    (bind _asbp_player (cast `/Game/Main/Blueprints/BP_Player` _returnvalue))
    (`PlayerCameraManager.StartCameraFade` :`self` (`GameplayStatics.GetPlayerCameraManager` 0) :`ToAlpha` 1.0 :`Duration` 1.0 :`bHoldWhenFinished` true)
    (`KismetSystemLibrary.Delay` 1.0)
    (`self.K2_TeleportTo` _asbp_player (`self.K2_GetActorLocation` _spawnpoint) (`self.K2_GetActorRotation` _spawnpoint))
    (`PlayerCameraManager.StartCameraFade` :`self` (`GameplayStatics.GetPlayerCameraManager` 0) :`FromAlpha` 1.0 :`ToAlpha` 0.0 :`Duration` 1.0 :`bHoldWhenFinished` true)))

(fn `UserConstructionScript`)